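; CARLA actor factory that publishes pedestrian definitions from its Walkers list and spawns walkers on request.
; SpawnActor creates the described pawn, gives it the WalkerController, and returns a spawn status.
; On BP_Walker pawns it sets invincibility and wheelchair use from description attributes, requiring both requested use and capability for wheelchairs.
; A separate event calls WheelchairAdd on a given walker after a short delay.
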(event `AddWheelchairToWalker`
  (params (WalkerChairToBeAssigned :type "/Game/Carla/Blueprints/Walkers/BP_Walker Object Reference"))
  (`KismetSystemLibrary.Delay` 0.6)
  (`/Game/Carla/Blueprints/Walkers/BP_Walker.WheelchairAdd` WalkerChairToBeAssigned))

(fn `GenerateDefinitions`
  (returns (ReturnValue :type "Array of ActorDefinition Structure"))
  (locals (Walkers :type "Array of PedestrianParameters Structure"))
  (bind _definitions (`ActorBlueprintFunctionLibrary.MakePedestrianDefinitions` (`local.Walkers`)))
  (bind _output_get (set `self.Definitions` _definitions))
  (return _output_get))

(fn `SpawnActor`
  (params (SpawnAtTransform :type "Transform Structure (by ref)") (ActorDescription :type "ActorDescription Structure (by ref)"))
  (returns (SpawnResult :type "ActorSpawnResult Structure"))
  (if (`KismetSystemLibrary.IsValidClass` ActorDescription_Class)
    (bind _returnvalue (`|SpawnActorFromClass` ActorDescription_Class SpawnAtTransform "Undefined" "OverrideRootScale" null null))
    (`/Engine/EditorBlueprintResources/StandardMacros.IsValid` _returnvalue
      (:`Is Valid`
        (bind _aspawn (cast `Pawn` _returnvalue)
          (:`then`
            (set `Pawn.AIControllerClass` "/Script/Carla.WalkerController" _aspawn)
            (`Pawn.SpawnDefaultController` _aspawn)
            (bind _asbp_walker (cast `/Game/Carla/Blueprints/Walkers/BP_Walker` _returnvalue)
              (:`then`
                (bind _returnvalue_2 (`ActorBlueprintFunctionLibrary.RetrieveActorAttributeToBool` "is_invincible" ActorDescription_Variations true))
                (set `/Game/Carla/Blueprints/Walkers/BP_Walker.bIsInvincible` _returnvalue_2 _asbp_walker)
                (bind _returnvalue_3 (`ActorBlueprintFunctionLibrary.RetrieveActorAttributeToBool` "use_wheelchair" ActorDescription_Variations))
                (bind _returnvalue_4 (`ActorBlueprintFunctionLibrary.RetrieveActorAttributeToBool` "can_use_wheelchair" ActorDescription_Variations))
                (set `WalkerBase.bUsesWheelChair` (and _returnvalue_3 _returnvalue_4) _asbp_walker)
                (return (make `ActorSpawnResult` _returnvalue "Success")))
              (:`CastFailed`
                (return (make `ActorSpawnResult` null)))))
          (:`CastFailed`
            (return (make `ActorSpawnResult` null)))))
      (:`Is Not Valid`
        (return (make `ActorSpawnResult` null "Collision"))))
    (else
      (return (make `ActorSpawnResult` null "InvalidDescription")))))

(fn `UserConstructionScript`)